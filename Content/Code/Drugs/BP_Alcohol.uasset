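; BP_Alcohol is a drug that, on activation, fires a damaging ranged shot from the player toward the mouse location.
; It runs a sphere trace against each demon's capsule, starting a capsule half-height from the player and reaching to Range, with persistent debug drawing.
; The first demon hit in array order, not necessarily the nearest, takes base damage scaled by Tolerance.
; It also exposes its drug type.
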(fn `ActivateDrug`
  (params (Player :type "/Game/Code/Characters/BP_Player Object Reference") (Demons :type "Array of /Game/Code/Characters/BP_Demon Object Reference (by ref)") (PlayerLocation :type "Vector Structure") (MouseLocation :type "Vector Structure") (Tolerance :type "Float (double-precision)"))
  (bind _returnvalue (`KismetMathLibrary.GetDirectionUnitVector` PlayerLocation MouseLocation))
  (for _array_element Demons
    (bind (_hitlocation _hitnormal _bonename _outhit _returnvalue_2) (`PrimitiveComponent.K2_SphereTraceComponent` (`Character.CapsuleComponent` _array_element) (`self.Offset Vector` PlayerLocation _returnvalue (`CapsuleComponent.CapsuleHalfHeight` (`Character.CapsuleComponent` Player))) (`self.Offset Vector` PlayerLocation _returnvalue (`self.Range`)) 50.0 true true true))
    (if _returnvalue_2
      (bind _asbp_demon (cast `/Game/Code/Characters/BP_Demon` (`.HitActor` (`GameplayStatics.BreakHitResult` _outhit))))
      (`/Game/Code/Characters/BP_Demon.TakeDamage` _asbp_demon (* Tolerance (`self.BaseDamage`)) _hitlocation)
      (break))))

(fn `GetType`
  (returns (DrugType :type "/Game/Code/Drugs/BP_DrugTypes Enum"))
  (return (`self.DrugType`)))

(fn `Offset Vector`
  (params (Location :type "Vector Structure") (Direction :type "Vector Structure") (Offset :type "Float (double-precision)"))
  (returns (ReturnValue :type "Vector Structure"))
  (return (+ Location (* Direction Offset))))