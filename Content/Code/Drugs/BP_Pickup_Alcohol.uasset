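; BP_Pickup_Alcohol is a pickup that gives the player an alcohol drug on overlap.
; When a BP_Player overlaps it, it prints a debug message, constructs a Drug object with the player as outer and stores it as CurrentDrug.
; It then copies its static mesh's first material onto the player's Body, visually marking the pickup, and destroys itself.
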(event `self.ReceiveActorBeginOverlap`
  (params (OtherActor :type "Actor Object Reference"))
  (bind _asbp_player (cast `/Game/Code/Characters/BP_Player` OtherActor))
  (`KismetSystemLibrary.PrintString` "Adding Alcohol")
  (bind _returnvalue (`|GenericCreateObject` (`self.Drug`) _asbp_player))
  (set `/Game/Code/Characters/BP_Player.CurrentDrug` _returnvalue _asbp_player)
  (`PrimitiveComponent.SetMaterial` (`/Game/Base/BP_BaseCharacter.Body` _asbp_player) 0 (`PrimitiveComponent.GetMaterial` (`self.StaticMesh`) 0))
  (`self.K2_DestroyActor`))

(fn `UserConstructionScript`
  (`parent.UserConstructionScript`))