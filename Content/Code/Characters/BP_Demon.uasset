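; BP_Demon is an enemy that hurts the player on contact and can be killed.
; When its Sphere begins overlapping a BP_Player, it subtracts its Damage directly from that player's Health.
; Its TakeDamage function sets Health to incoming Damage minus current Health (operands reversed from a usual subtraction).
; At zero or below, it spawns a PS_Poof emitter at the hit location and destroys the actor.
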(event `self.ReceiveActorBeginOverlap`
  (params (OtherActor :type "Actor Object Reference")))

(event `self.Sphere.OnComponentBeginOverlap`
  (params (OverlappedComponent :type "PrimitiveComponent Object Reference") (OtherActor :type "Actor Object Reference") (OtherComp :type "PrimitiveComponent Object Reference") (OtherBodyIndex :type Integer) (bFromSweep :type Boolean) (SweepResult :type "HitResult Structure (by ref)"))
  (bind _asbp_player (cast `/Game/Code/Characters/BP_Player` OtherActor))
  (set `/Game/Code/Characters/BP_Player.Health` (- (`/Game/Code/Characters/BP_Player.Health` _asbp_player) (`self.Damage`)) _asbp_player))

(fn `TakeDamage`
  (params (Damage :type "Float (double-precision)") (HitLocation :type "Vector Structure"))
  (bind _output_get (set `self.Health` (- Damage (`self.Health`))))
  (if (<= _output_get 0.0)
    (`GameplayStatics.SpawnEmitterAtLocation` "/Game/Data/ParticleEffects/PS_Poof.PS_Poof" HitLocation)
    (`self.K2_DestroyActor`)))

(fn `UserConstructionScript`
  (`parent.UserConstructionScript`))